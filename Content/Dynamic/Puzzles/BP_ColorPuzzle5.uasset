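; BP_ColorPuzzle5 is a color puzzle layout with five buttons and six slots.
; Its Construction Script fills the Buttons and Slots arrays and starts each button in its numbered slot, leaving Slot0 without a button.
; It then defines slot adjacency as a hub and ring: Slot0 neighbors every other slot, and Slots 1 to 5 form a closed loop around it.
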(fn ConstructionScript
  (Utilities|FlowControl|Sequence
    (:then_0
      ;[1 1 1] Set buttons and slots arrays
      (Variables|Default|SetButtons (Utilities|Array|MakeArray (Variables|Default|GetBP_ColorPuzzleButton1) (Variables|Default|GetBP_ColorPuzzleButton2) (Variables|Default|GetBP_ColorPuzzleButton3) (Variables|Default|GetBP_ColorPuzzleButton4) (Variables|Default|GetBP_ColorPuzzleButton5)))
      (Variables|Default|SetSlots (Utilities|Array|MakeArray (Variables|Default|GetBP_ColorPuzzleSlot0) (Variables|Default|GetBP_ColorPuzzleSlot1) (Variables|Default|GetBP_ColorPuzzleSlot2) (Variables|Default|GetBP_ColorPuzzleSlot3) (Variables|Default|GetBP_ColorPuzzleSlot4) (Variables|Default|GetBP_ColorPuzzleSlot5))))
    (:then_1
      ;[1 1 1] Set starting button slots
      (Utilities|FlowControl|Sequence
        (:then_0
          (Variables|/Script/DeeperAndDeeper.ColorPuzzleButton|SetSlot (Variables|Default|GetBP_ColorPuzzleButton1) (Variables|Default|GetBP_ColorPuzzleSlot1)))
        (:then_1
          (Variables|/Script/DeeperAndDeeper.ColorPuzzleButton|SetSlot (Variables|Default|GetBP_ColorPuzzleButton2) (Variables|Default|GetBP_ColorPuzzleSlot2)))
        (:then_2
          (Variables|/Script/DeeperAndDeeper.ColorPuzzleButton|SetSlot (Variables|Default|GetBP_ColorPuzzleButton3) (Variables|Default|GetBP_ColorPuzzleSlot3)))
        (:then_3
          (Variables|/Script/DeeperAndDeeper.ColorPuzzleButton|SetSlot (Variables|Default|GetBP_ColorPuzzleButton4) (Variables|Default|GetBP_ColorPuzzleSlot4)))
        (:then_4
          (Variables|/Script/DeeperAndDeeper.ColorPuzzleButton|SetSlot (Variables|Default|GetBP_ColorPuzzleButton5) (Variables|Default|GetBP_ColorPuzzleSlot5)))))
    (:then_2
      ;[1 1 1] Set slot neighbors
      (Variables|/Script/DeeperAndDeeper.ColorPuzzleSlot|SetNeighborSlots (Variables|Default|GetBP_ColorPuzzleSlot0) (Utilities|Array|MakeArray (Variables|Default|GetBP_ColorPuzzleSlot1) (Variables|Default|GetBP_ColorPuzzleSlot2) (Variables|Default|GetBP_ColorPuzzleSlot3) (Variables|Default|GetBP_ColorPuzzleSlot4) (Variables|Default|GetBP_ColorPuzzleSlot5)))
      (Variables|/Script/DeeperAndDeeper.ColorPuzzleSlot|SetNeighborSlots (Variables|Default|GetBP_ColorPuzzleSlot1) (Utilities|Array|MakeArray (Variables|Default|GetBP_ColorPuzzleSlot0) (Variables|Default|GetBP_ColorPuzzleSlot2) (Variables|Default|GetBP_ColorPuzzleSlot5)))
      (Variables|/Script/DeeperAndDeeper.ColorPuzzleSlot|SetNeighborSlots (Variables|Default|GetBP_ColorPuzzleSlot2) (Utilities|Array|MakeArray (Variables|Default|GetBP_ColorPuzzleSlot0) (Variables|Default|GetBP_ColorPuzzleSlot1) (Variables|Default|GetBP_ColorPuzzleSlot3)))
      (Variables|/Script/DeeperAndDeeper.ColorPuzzleSlot|SetNeighborSlots (Variables|Default|GetBP_ColorPuzzleSlot3) (Utilities|Array|MakeArray (Variables|Default|GetBP_ColorPuzzleSlot0) (Variables|Default|GetBP_ColorPuzzleSlot2) (Variables|Default|GetBP_ColorPuzzleSlot4)))
      (Variables|/Script/DeeperAndDeeper.ColorPuzzleSlot|SetNeighborSlots (Variables|Default|GetBP_ColorPuzzleSlot4) (Utilities|Array|MakeArray (Variables|Default|GetBP_ColorPuzzleSlot0) (Variables|Default|GetBP_ColorPuzzleSlot3) (Variables|Default|GetBP_ColorPuzzleSlot5)))
      (Variables|/Script/DeeperAndDeeper.ColorPuzzleSlot|SetNeighborSlots (Variables|Default|GetBP_ColorPuzzleSlot5) (Utilities|Array|MakeArray (Variables|Default|GetBP_ColorPuzzleSlot0) (Variables|Default|GetBP_ColorPuzzleSlot4) (Variables|Default|GetBP_ColorPuzzleSlot1))))))