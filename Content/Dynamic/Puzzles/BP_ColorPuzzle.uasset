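; BP_ColorPuzzle is a puzzle actor made of four color buttons and five slots.
; Its construction script collects them into Buttons and Slots arrays and places the buttons in slots 1 to 4, leaving slot 0 empty.
; It also builds the slot adjacency graph through each slot's NeighborSlots: slot 0 links to all others, while slots 1 to 4 form a ring around it.
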(fn ConstructionScript
  (Utilities|FlowControl|Sequence
    (:then_0
      ;[1 1 1] Set buttons and slots arrays
      (Variables|Default|SetButtons (Utilities|Array|MakeArray (Variables|Default|GetBP_ColorPuzzleButton0) (Variables|Default|GetBP_ColorPuzzleButton1) (Variables|Default|GetBP_ColorPuzzleButton2) (Variables|Default|GetBP_ColorPuzzleButton3)))
      (Variables|Default|SetSlots (Utilities|Array|MakeArray (Variables|Default|GetBP_ColorPuzzleSlot0) (Variables|Default|GetBP_ColorPuzzleSlot1) (Variables|Default|GetBP_ColorPuzzleSlot2) (Variables|Default|GetBP_ColorPuzzleSlot3) (Variables|Default|GetBP_ColorPuzzleSlot4))))
    (:then_1
      ;[1 1 1] Set starting button slots
      (Utilities|FlowControl|Sequence
        (:then_0
          (Variables|/Script/DeeperAndDeeper.ColorPuzzleButton|SetSlot (Variables|Default|GetBP_ColorPuzzleButton0) (Variables|Default|GetBP_ColorPuzzleSlot1)))
        (:then_1
          (Variables|/Script/DeeperAndDeeper.ColorPuzzleButton|SetSlot (Variables|Default|GetBP_ColorPuzzleButton1) (Variables|Default|GetBP_ColorPuzzleSlot2)))
        (:then_2
          (Variables|/Script/DeeperAndDeeper.ColorPuzzleButton|SetSlot (Variables|Default|GetBP_ColorPuzzleButton2) (Variables|Default|GetBP_ColorPuzzleSlot3)))
        (:then_3
          (Variables|/Script/DeeperAndDeeper.ColorPuzzleButton|SetSlot (Variables|Default|GetBP_ColorPuzzleButton3) (Variables|Default|GetBP_ColorPuzzleSlot4)))))
    (:then_2
      ;[1 1 1] Set slot neighbors
      (Utilities|FlowControl|Sequence
        (:then_0
          (Variables|/Script/DeeperAndDeeper.ColorPuzzleSlot|SetNeighborSlots (Variables|Default|GetBP_ColorPuzzleSlot0) (Utilities|Array|MakeArray (Variables|Default|GetBP_ColorPuzzleSlot1) (Variables|Default|GetBP_ColorPuzzleSlot2) (Variables|Default|GetBP_ColorPuzzleSlot3) (Variables|Default|GetBP_ColorPuzzleSlot4))))
        (:then_1
          (Variables|/Script/DeeperAndDeeper.ColorPuzzleSlot|SetNeighborSlots (Variables|Default|GetBP_ColorPuzzleSlot1) (Utilities|Array|MakeArray (Variables|Default|GetBP_ColorPuzzleSlot0) (Variables|Default|GetBP_ColorPuzzleSlot2) (Variables|Default|GetBP_ColorPuzzleSlot4))))
        (:then_2
          (Variables|/Script/DeeperAndDeeper.ColorPuzzleSlot|SetNeighborSlots (Variables|Default|GetBP_ColorPuzzleSlot2) (Utilities|Array|MakeArray (Variables|Default|GetBP_ColorPuzzleSlot0) (Variables|Default|GetBP_ColorPuzzleSlot1) (Variables|Default|GetBP_ColorPuzzleSlot3))))
        (:then_3
          (Variables|/Script/DeeperAndDeeper.ColorPuzzleSlot|SetNeighborSlots (Variables|Default|GetBP_ColorPuzzleSlot3) (Utilities|Array|MakeArray (Variables|Default|GetBP_ColorPuzzleSlot0) (Variables|Default|GetBP_ColorPuzzleSlot2) (Variables|Default|GetBP_ColorPuzzleSlot4))))
        (:then_4
          (Variables|/Script/DeeperAndDeeper.ColorPuzzleSlot|SetNeighborSlots (Variables|Default|GetBP_ColorPuzzleSlot4) (Utilities|Array|MakeArray (Variables|Default|GetBP_ColorPuzzleSlot0) (Variables|Default|GetBP_ColorPuzzleSlot1) (Variables|Default|GetBP_ColorPuzzleSlot3))))))))